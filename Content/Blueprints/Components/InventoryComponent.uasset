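; Inventory component that stores items as stacks with class, UI offset, size and tag data, under a weight limit.
; Pickups from actors or stacks auto-merge into same-class stacks with identical tags up to the class's max size, otherwise becoming new entries.
; Events split, move, merge, remove and drop stacks, with drops respawning actors from stack data.
; Changes update visible UI_Inventory widgets linked to this component through AddItem or PopulatePanel.
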(event Custom|AddItemStackFromItemStack
  (params (ItemToPickup :type Item%20Stack%20Structure) (AutoPlace :type Boolean))
  ;[1 1 1] Add an item to the inventory; either from an existing actor (which is then converted to a stack) or directly from a stack
  (bind (_success _stack _index _newstack) (Manipulation|AddandMergeStacks 0 ItemToPickup AutoPlace))
  (if (and _success _newstack)
    (CallFunction|AddItemUI _index)))

(event Custom|SplitItemStack
  (params (StackIndex :type Integer) (GetSingle :type Boolean))
  (bind _inventory (Variables|Default|GetInventory))
  (bind _inventory_2 (Variables|Default|GetInventory))
  (bind _output (Utilities|Array|Get(acopy) _inventory StackIndex))
  (bind _output_2 (Utilities|Array|Get(acopy) _inventory_2 StackIndex))
  (bind _returnvalue (/ (.stacksize _output) 2))
  ;[1 1 1] Comment
  (if GetSingle
    (bind _returnvalue_2 (Utilities|Array|Add _inventory_2 (Utilities|Struct|MakeItemStack (.actorclass _output_2) (.stacklocationoffset _output_2) (- (.stacksize _output_2) 1) (.tagdata _output_2))))
    (Utilities|Array|SetArrayElem _inventory_2 StackIndex (Utilities|Struct|MakeItemStack (.actorclass _output_2) (.stacklocationoffset _output_2) 1 (.tagdata _output_2)))
    (CallFunction|AddItemUI _returnvalue_2)
    (else
      (bind _returnvalue_3 (Utilities|Array|Add _inventory (Utilities|Struct|MakeItemStack (.actorclass _output) (.stacklocationoffset _output) (- (.stacksize _output) _returnvalue) (.tagdata _output))))
      (Utilities|Array|SetArrayElem _inventory StackIndex (Utilities|Struct|MakeItemStack (.actorclass _output) (.stacklocationoffset _output) _returnvalue (.tagdata _output)))
      (CallFunction|AddItemUI _returnvalue_3))))

(event Custom|ToggleCharacterInteraction
  (params (Character :type RPG%20Character%20Object%20Reference) (Add :type Boolean))
  (bind _interactingcharacters (Variables|Default|GetInteractingCharacters))
  ;[1 1 1] server only
  ;;[1 1 1] Add or subtract a player from the list of players currently interacting with this container; this helps us determine if players need to be notified of changes
  (if Add
    (Utilities|Array|Add _interactingcharacters Character)
    (else
      (Utilities|Array|RemoveItem _interactingcharacters Character))))

(event Custom|MoveItemStack
  (params (StackIndex :type Integer) (StackOffset :type Vector%202D%20Structure) (MergeIndex :type Integer))
  (bind _inventory (Variables|Default|GetInventory))
  (bind _output (Utilities|Array|Get(acopy) _inventory StackIndex))
  ;[1 1 1] server only
  ;;[1 1 1] Set the localized (to it's inventory UI) offset of an inventory item to the provided offset
  (Utilities|Array|SetArrayElem _inventory StackIndex (Utilities|Struct|MakeItemStack (.actorclass _output) StackOffset (.stacksize _output) (.tagdata _output)) true)
  (if (not (== MergeIndex -1))
    (CallFunction|MergeItemStacks MergeIndex StackIndex)))

(event Custom|RefreshUI
  ;[1 1 1] Run on all clients; all clients will iterate through their open inventories and update the panels if they exist and are linked to this inventory
  (bind _foundwidgets (Widget|GetAllWidgetsOfClass "/Game/Blueprints/UI/UI_Inventory.UI_Inventory_C" false))
  (for _array_element _foundwidgets
    (if (and (== (Variables|/Game/Blueprints/UI/UI_Inventory.UI_Inventory_C|GetLinkedInventory _array_element) self) (Widget|IsVisible _array_element))
      (Default|PopulatePanel _array_element))))

(event Custom|AddItemStackFromActor
  (params (ItemToPickup :type Item%20Base%20Object%20Reference))
  ;[1 1 1] Add an item to the inventory; either from an existing actor (which is then converted to a stack) or directly from a stack
  (bind (_success _stack _index _newstack) (Manipulation|AddandMergeStacks :ItemBase ItemToPickup :AutoPlace true))
  (if _success
    (if _newstack
      (CallFunction|AddItemUI _index))
    (Class|IInteractableEntity|OnItemPickup(Message) ItemToPickup)))

(event Custom|DropItemStack
  (params (StackIndex :type Integer) (WorldVector :type Vector))
  (bind _inventory (Variables|Default|GetInventory))
  (bind _output (Utilities|Array|Get(acopy) _inventory StackIndex))
  ;[1 1 1] server only
  ;;[1 1 1] Spawn an item in the world with a given vector and then remove the item from the stack
  (bind _returnvalue (Game|SpawnActorfromClass (.ActorClass (Utilities|Struct|BreakItemStack _output)) (Math|Transform|MakeTransform WorldVector "0, 0, 0" "1,1,1") "Undefined" 0 0))
  (Default|DecompressfromStack _returnvalue _output)
  (CallFunction|RemoveItemStack StackIndex))

(event Custom|MergeItemStacks
  (params (IndexToAddTo :type Integer) (IndexToAddFrom :type Integer))
  ;[1 1 1] server only
  (Manipulation|ManuallyMergeStacks IndexToAddTo IndexToAddFrom))

(event Custom|RemoveItemStack
  (params (StackIndex :type Integer))
  (bind _inventory (Variables|Default|GetInventory))
  ;[1 1 1] server only
  ;;[1 1 1] Remove the selected item from the inventory at provided index
  (bind _weight (Utility|GetStackWeight (Utilities|Array|Get(acopy) _inventory StackIndex)))
  (Variables|Default|SetWeightCurrent (- (Variables|Default|GetWeightCurrent) _weight))
  (Utilities|Array|RemoveIndex _inventory StackIndex)
  (CallFunction|RefreshUI))

(event Custom|InitializeInventory
  ;[1 1 1] server only
  ;;[0 0 0] This primarily takes the content that may exist as data before this actor actually exists and updates the actor's variables; at the moment, only necessary to increase the combined weight of the components contents
  (for _array_element (Variables|Default|GetInventory)
    (bind _weight (Utility|GetStackWeight _array_element))
    (Variables|Default|SetWeightCurrent (+ _weight (Variables|Default|GetWeightCurrent)))))

(event Custom|AddItemUI
  (params (Index :type Integer))
  ;[1 1 1] Run on all clients; all clients will iterate through their open inventories and update the panels if they exist and are linked to this inventory
  (bind _foundwidgets (Widget|GetAllWidgetsOfClass "/Game/Blueprints/UI/UI_Inventory.UI_Inventory_C" false))
  (for _array_element _foundwidgets
    (if (and (== (Variables|/Game/Blueprints/UI/UI_Inventory.UI_Inventory_C|GetLinkedInventory _array_element) self) (Widget|IsVisible _array_element))
      (Default|AddItem _array_element Index))))

(fn AreTagsEqual
  (params (TagA :type Map%20of%20Names%20to%20Strings) (TagB :type Map%20of%20Names%20to%20Strings))
  ;[1 1 1] This function is used to determine if two stacks should be able to combine, as data tags must be IDENTICAL
  (bind _keys (Utilities|Map|Keys TagA))
  (bind _array_element (Utilities|Array|ForEachLoopwithBreak _keys :!label _label)
    (:LoopBody
      (if (.ReturnValue (Utilities|Map|Find TagA _array_element))
        (if (not (Utilities|Enum|Equal(Enum) (.Value (Utilities|Map|Find TagB _array_element)) (.Value (Utilities|Map|Find TagA _array_element))))
          (LocalVariables|SetFailedFind true)
          (goto _label Break))
        (else
          (LocalVariables|SetFailedFind true)
          (goto _label Break))))
    (:Completed
      (return (not (LocalVariables|GetFailedFind))))))

(fn AddandMergeStacks
  (params (ItemBase :type Item%20Base%20Object%20Reference) (ItemStack :type Item%20Stack%20Structure) (AutoPlace :type Boolean))
  ;[1 1 1] Convert an actor to an itemstack, then ensure that the itemstack weighs less than the max weight of our inventory
  (Utilities|IsValid ItemBase
    (:Is%20Valid
      (bind _itemstack (Default|CompresstoStack ItemBase))
      (LocalVariables|SetTempInventoryItem _itemstack))
    (:Is%20Not%20Valid
      (LocalVariables|SetTempInventoryItem ItemStack)))
  (bind _canfit (Utility|DoesInventoryHaveRoom (LocalVariables|GetTempInventoryItem)))
  (if _canfit
    (if AutoPlace
      ;[1 1 1] For all of our items, check if there exists an itemstack that our newly added item may potentially stack onto; tags must be identical
      (bind (_array_element _array_index) (Utilities|Array|ForEachLoopwithBreak (Variables|Default|GetInventory) :!label _label)
        (:LoopBody
          ;[1 1 1] If we find a stack that has the same class, check if we have identical tags; additionally, if the stack size we're adding is larger than the max stack size of the potential stack, go ahead and repeat this process
          (LocalVariables|SetFoundExistingItem false)
          (LocalVariables|SetRemainderRemoval 0)
          (if (== (.ActorClass (Utilities|Struct|BreakItemStack _array_element)) (.actorclass (LocalVariables|GetTempInventoryItem)))
            (if (not (>= (.StackSize (Utilities|Struct|BreakItemStack _array_element)) (Utilities|GetClassDefaults (.actorclass (LocalVariables|GetTempInventoryItem)))))
              (if (<= (+ (.StackSize (Utilities|Struct|BreakItemStack _array_element)) (.stacksize (LocalVariables|GetTempInventoryItem))) (Utilities|GetClassDefaults (.actorclass (LocalVariables|GetTempInventoryItem))))
                _
                (else
                  (LocalVariables|SetRemainderRemoval (- (+ (.StackSize (Utilities|Struct|BreakItemStack _array_element)) (.stacksize (LocalVariables|GetTempInventoryItem))) (Utilities|GetClassDefaults (.actorclass (LocalVariables|GetTempInventoryItem)))))))
              (bind _equaltags (Utility|AreTagsEqual (.TagData (Utilities|Struct|BreakItemStack _array_element)) (.tagdata (LocalVariables|GetTempInventoryItem))))
              (if _equaltags
                (LocalVariables|SetFoundExistingItem true)
                (LocalVariables|SetArrayIndex _array_index)
                (goto _label Break)
                (else
                  (Development|PrintString "uneqal tags"))))))
        (:Completed
          ;[1 1 1] If we found an identical item, add to stack
          (if (LocalVariables|GetFoundExistingItem)
            ;[1 1 1] If this stack does not fully go into one of the existing stacks, (remainderremoval>0) then set the found index to the max size (class defaults), set the temp item to the remainder, and repeat the process
            (if (== (LocalVariables|GetRemainderRemoval) 0)
              ;[1 1 1] Once we have no more remainders left, go ahead and fill up another stack
              (bind _weight (Utility|GetStackWeight (LocalVariables|GetTempInventoryItem)))
              (LocalVariables|SetWeightToAdd _weight)
              (bind _output_get (LocalVariables|SetTempInventoryItem (Utilities|Struct|MakeItemStack (.actorclass (Utilities|Array|Get(acopy) (Variables|Default|GetInventory) (LocalVariables|GetArrayIndex))) (.stacklocationoffset (Utilities|Array|Get(acopy) (Variables|Default|GetInventory) (LocalVariables|GetArrayIndex))) (+ (.stacksize (LocalVariables|GetTempInventoryItem)) (.stacksize (Utilities|Array|Get(acopy) (Variables|Default|GetInventory) (LocalVariables|GetArrayIndex)))) (.tagdata (Utilities|Array|Get(acopy) (Variables|Default|GetInventory) (LocalVariables|GetArrayIndex))))))
              (Utilities|Array|SetArrayElem (Variables|Default|GetInventory) (LocalVariables|GetArrayIndex) _output_get true)
              (Variables|Default|SetWeightCurrent (+ (Variables|Default|GetWeightCurrent) (LocalVariables|GetWeightToAdd)))
              (return true (LocalVariables|GetTempInventoryItem) (LocalVariables|GetArrayIndex) false)
              (else
                (bind _output_get_2 (LocalVariables|SetTempInventoryItem (Utilities|Struct|MakeItemStack (.ActorClass (Utilities|Struct|BreakItemStack (LocalVariables|GetTempInventoryItem))) (.StackLocationOffset (Utilities|Struct|BreakItemStack (LocalVariables|GetTempInventoryItem))) (- (.StackSize (Utilities|Struct|BreakItemStack (LocalVariables|GetTempInventoryItem))) (LocalVariables|GetRemainderRemoval)) (.TagData (Utilities|Struct|BreakItemStack (LocalVariables|GetTempInventoryItem))))))
                (bind _weight_2 (Utility|GetStackWeight _output_get_2))
                (LocalVariables|SetWeightToAdd _weight_2)
                (Utilities|Array|SetArrayElem (Variables|Default|GetInventory) (LocalVariables|GetArrayIndex) _output_get_2 true)
                (Variables|Default|SetWeightCurrent (+ (Variables|Default|GetWeightCurrent) (LocalVariables|GetWeightToAdd)))
                (LocalVariables|SetTempInventoryItem (Utilities|Struct|MakeItemStack (.actorclass (LocalVariables|GetTempInventoryItem)) (.stacklocationoffset (LocalVariables|GetTempInventoryItem)) (LocalVariables|GetRemainderRemoval) (.tagdata (LocalVariables|GetTempInventoryItem))))
                (goto _label)))
            (else
              ;[1 1 1] If we don't have any existing stacks to plop into, add a new entry in the array
              (bind _returnvalue (Utilities|Array|Add (Variables|Default|GetInventory) (LocalVariables|GetTempInventoryItem) :!label _label_2))
              (bind _weight_3 (Utility|GetStackWeight (LocalVariables|GetTempInventoryItem)))
              (bind _output_get_3 (LocalVariables|SetWeightToAdd _weight_3))
              (Variables|Default|SetWeightCurrent (+ _output_get_3 (Variables|Default|GetWeightCurrent)))
              (return true (LocalVariables|GetTempInventoryItem) _returnvalue true)))))
      (else
        (goto _label_2)))
    (else
      (return false "" -1 false))))

(fn GetStackWeight
  (params (Stack :type Item%20Stack%20Structure))
  (bind (_actorclass _stacklocationoffset _stacksize _tagdata) (Utilities|Struct|BreakItemStack Stack))
  (bind (_value _returnvalue) (Utilities|Map|Find _tagdata "weight"))
  (bind _weightbase (Utilities|GetClassDefaults _actorclass))
  (if _returnvalue
    (return (* _stacksize (+ _weightbase (Math|Conversions|ToFloat(Integer) _value))))
    (else
      (return (* _stacksize _weightbase)))))

(fn DoesInventoryHaveRoom
  (params (ItemStack :type Item%20Stack%20Structure))
  (bind _output_get (LocalVariables|SetTemporaryStack ItemStack))
  (bind _weight (Utility|GetStackWeight _output_get))
  (if (<= (+ (Variables|Default|GetWeightCurrent) _weight) (Variables|Default|GetWeightMax))
    (return true _weight)
    (else
      (return false _weight))))

(fn GetStacksMergeable
  (params (FromIndex :type Integer) (ToIndex :type Integer))
  (bind _inventory (Variables|Default|GetInventory))
  (bind _output (Utilities|Array|Get(acopy) _inventory FromIndex))
  (bind _output_2 (Utilities|Array|Get(acopy) _inventory ToIndex))
  (if (== (.actorclass _output) (.actorclass _output_2))
    (if (< (.stacksize _output_2) (Utilities|GetClassDefaults (.actorclass _output_2)))
      (bind _equaltags (Utility|AreTagsEqual (.tagdata _output) (.tagdata _output_2)))
      (return _equaltags)
      (else
        _)))
  (return false))

(fn ManuallyMergeStacks
  (params (FromIndex :type Integer) (ToIndex :type Integer))
  (bind _inventory (Variables|Default|GetInventory))
  (bind _inventory_2 (Variables|Default|GetInventory))
  (bind _output (Utilities|Array|Get(acopy) _inventory_2 ToIndex))
  (bind _output_2 (Utilities|Array|Get(acopy) _inventory FromIndex))
  (bind _output_3 (Utilities|Array|Get(acopy) _inventory ToIndex))
  (bind _output_4 (Utilities|Array|Get(acopy) _inventory_2 FromIndex))
  (bind _returnvalue (+ (.stacksize _output_4) (.stacksize _output)))
  (bind _stacksizemax (Utilities|GetClassDefaults (.actorclass _output_4)))
  (if (> _returnvalue _stacksizemax)
    (LocalVariables|SetRemainderStack (- _returnvalue _stacksizemax))
    (Utilities|Array|SetArrayElem _inventory FromIndex (Utilities|Struct|MakeItemStack (.actorclass _output_2) (.stacklocationoffset _output_2) _stacksizemax (.tagdata _output_2)))
    (Utilities|Array|SetArrayElem _inventory ToIndex (Utilities|Struct|MakeItemStack (.actorclass _output_3) (.stacklocationoffset _output_3) (LocalVariables|GetRemainderStack) (.tagdata _output_3)))
    (else
      (Utilities|Array|SetArrayElem _inventory_2 FromIndex (Utilities|Struct|MakeItemStack (.actorclass _output_4) (.stacklocationoffset _output_4) _returnvalue (.tagdata _output_4)))
      (Utilities|Array|RemoveIndex _inventory_2 ToIndex)
      (CallFunction|RefreshUI))))