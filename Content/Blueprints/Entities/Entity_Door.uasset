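; Interactable door entity that players can open, close, lock and unlock through a default interaction or context actions.
; PerformAction routes actions to a lock toggle or ToggleDoor, a multicast that eases the rotation point between open and closed transforms while the authority updates state.
; Available context actions are filtered by open and locked state, and interaction is blocked while moving.
; Locking has no key check yet, and damage is ignored.
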(event Custom|ToggleLock
  ;[1 1 1] Currently we don't check to see if the player has keys or anything
  (bind _output_get (Variables|Default|SetIsLocked (not (Variables|Default|GetIsLocked))))
  (Development|PrintString (Utilities|String|ToString(Boolean) _output_get)))

(event Custom|ToggleDoor
  (params (User :type Actor%20Object%20Reference))
  (bind _closedrelativetransform (Variables|Default|GetClosedRelativeTransform))
  (bind _movementspeed (Variables|Default|GetMovementSpeed))
  (bind _openrelativetransform (Variables|Default|GetOpenRelativeTransform))
  (bind _doorrotationpoint (Variables|Default|GetDoorRotationPoint))
  ;[1 1 1] Multicast door status change; if server, set serverside state vars, if client (or listen server) most component over time to open/close position
  (Networking|SwitchHasAuthority
    (:Authority
      (Variables|Default|SetIsMoving true))
    (:Remote
      _))
  (if (Variables|Default|GetIsOpen)
    (Components|MoveComponentTo _doorrotationpoint (.location _closedrelativetransform) (.rotation _closedrelativetransform) false true _movementspeed false)
    (else
      (Components|MoveComponentTo _doorrotationpoint (.location _openrelativetransform) (.rotation _openrelativetransform) true true _movementspeed false)))
  (Networking|SwitchHasAuthority
    (:Authority
      (Variables|Default|SetIsOpen (not (Variables|Default|GetIsOpen)))
      (Variables|Default|SetIsMoving false))))

(event EventPerformAction
  (params (User :type Actor%20Object%20Reference) (Action :type Name :default "None"))
  (bind _ismoving (Variables|Default|GetIsMoving))
  (bind _returnvalue (not _ismoving))
  ;[1 1 1] Switch on context action
  (switch name Action
    (:unlock
      (if (and _returnvalue (not (Variables|Default|GetIsOpen))) :!label _label
        (CallFunction|ToggleLock)))
    (:lock
      (goto _label))
    (:open
      (if (and (not (Variables|Default|GetIsLocked)) _returnvalue) :!label _label_2
        (CallFunction|ToggleDoor User)))
    (:close
      (goto _label_2))))

(event EventOnInteract
  (params (User :type Actor%20Object%20Reference))
  (bind _self self)
  ;[1 1 1] Default action: open or close door
  (if (and (not (Variables|Default|GetIsLocked)) (not (Variables|Default|GetIsMoving)))
    (Default|PerformAction _self User "close")
    (else
      (Default|PerformAction _self User "open"))))

(fn ConstructionScript)

(fn CanToggleDoor
  (return (and (not (Variables|Default|GetIsLocked)) (not (Variables|Default|GetIsMoving)))))

(fn DamageEntity
  (params (Location :type Vector :default "0, 0, 0") (Component :type Primitive%20Component%20Object%20Reference) (Damage :type Weapon%20Damage%20Structure) (Damager :type Actor%20Object%20Reference) (EquipmentSlot :type EquipmentSlot%20Enum :default "NewEnumerator0"))
  (return false))

(fn GetContextActions
  (params (Player :type RPG%20Character%20Object%20Reference))
  (LocalVariables|SetEditedCopy (Variables|Default|GetContextActions))
  (if (not (Variables|Default|GetIsMoving))
    (if (Variables|Default|GetIsOpen)
      (Utilities|Map|Remove (LocalVariables|GetEditedCopy) "open")
      (Utilities|Map|Remove (LocalVariables|GetEditedCopy) "lock")
      (Utilities|Map|Remove (LocalVariables|GetEditedCopy) "unlock")
      (Utilities|Map|Remove (LocalVariables|GetEditedCopy) "knock")
      (else
        (Utilities|Map|Remove (LocalVariables|GetEditedCopy) "close")
        (if (Variables|Default|GetIsLocked)
          (Utilities|Map|Remove (LocalVariables|GetEditedCopy) "lock")
          (Utilities|Map|Remove (LocalVariables|GetEditedCopy) "open")
          (else
            (Utilities|Map|Remove (LocalVariables|GetEditedCopy) "unlock")))))
    (return (LocalVariables|GetEditedCopy))))

(fn GetDisplayText
  (return "Door"))

(fn GetIneractable
  ;[1 1 1] We currently only check to see if the door is moving to determine whether we can open a context menu
  (return (not (Variables|Default|GetIsMoving))))