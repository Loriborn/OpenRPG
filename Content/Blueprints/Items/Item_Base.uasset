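; Base world item actor that players can inspect, pick up or equip through interaction and context actions.
; Pickup adds the item to the user's inventory, and equipping hands the actor and its stack to the RPG character.
; Converts to and from item stacks of class, size and tag data, with stubbed tag decompression and damage functions.
; Selection outline is a runtime-spawned mesh copy using a highlight material.
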(event Custom|UseItem
  (params (UsingActor :type Actor%20Object%20Reference))
  (Development|PrintString (Utilities|GetDisplayName UsingActor)))

(event Custom|EquipItem
  (params (Interactor :type Actor%20Object%20Reference))
  (bind _self self)
  (bind _asrpgcharacter (Utilities|Casting|CastToRPGCharacter Interactor))
  (Default|OnItemPickedUp _asrpgcharacter _self)
  (bind _itemstack (CallFunction|CompresstoStack))
  (Default|EquipItem _asrpgcharacter _self _itemstack))

(event Custom|PickupItem
  (params (User :type Actor%20Object%20Reference))
  (bind _self self)
  (bind _asrpgcharacter (Utilities|Casting|CastToRPGCharacter User)
    (:then
      (Default|OnItemPickedUp _asrpgcharacter _self)
      (Default|AddItemStackfromActor (Variables|/Game/Blueprints/Player/RPGCharacter.RPGCharacter_C|GetInventory _asrpgcharacter) _self))
    (:CastFailed
      (Default|AddItemStackfromActor (Actor|GetComponentbyClass User "/Game/Blueprints/Components/InventoryComponent.InventoryComponent_C") _self))))

(event EventPerformAction
  (params (User :type Actor%20Object%20Reference) (Action :type Name :default "None"))
  (switch name Action
    (:inspect
      (Development|PrintString "looks like a thing"))
    (:pickup
      (CallFunction|PickupItem User))
    (:equip
      (CallFunction|EquipItem User))))

(event EventToggleOutline
  (params (NewState :type Boolean))
  (if NewState
    (Utilities|IsValid (Variables|Default|GetSelectionMesh)
      (:Is%20Not%20Valid
        (bind _returnvalue (AddComponent|AddStaticMeshComponent false))
        (Components|StaticMesh|SetStaticMesh _returnvalue (Variables|/Script/Engine.StaticMeshComponent|GetStaticMesh (Variables|Default|GetItemMesh)))
        (Rendering|Material|SetMaterial _returnvalue 0 "/Game/Assets/Materials/Utility/Utility_Selection.Utility_Selection")
        (Variables|Default|SetSelectionMesh _returnvalue)))
    (else
      (Components|DestroyComponent (Variables|Default|GetSelectionMesh)))))

(event EventOnInteract
  (params (User :type Actor%20Object%20Reference))
  (CallFunction|PickupItem User))

(event EventBeginPlay
  (CallFunction|DecompressTags (Variables|Default|GetTagData)))

(event EventOnItemPickup
  (Actor|DestroyActor))

(fn ConstructionScript)

(fn DecompressTags
  (params (TagData :type Map%20of%20Names%20to%20Strings)))

(fn CompresstoStack
  ;[1 1 1] To - Do : All items will need to determine, on a per item class basis, what variables will need to be added to the tag data map; this would be any variable that persists after conversion to an itemstack, and is changed during run time. Not all variables need to be stored as tag data. We can also check if a variable is different from "class default" to determine whether it needs to be stored, rather than having a "modified" variable duplicate of the original; in this case, we can override base stats if we presume that we will not normally need the default class variable value in most circumstances. For instance, we would store a weapon's 'durability' but not its 'max_durability' as we can presume that normal gameplay would not result in the max durability of an item being altered during gameplay; if max durability CAN be altered during gameplay, ie. via some kind of enchantment or modifier component, we should specifically break that tag data on the individual item that can have its max durability modified. We can use the "add call to parent function" system to have each child actor search its respective data tags. The base items, I believe, only need to worry about name, and weight, but we can alter this later.
  (return (Utilities|Struct|MakeItemStack (Utilities|GetClass self) "(X=0.000000,Y=0.000000)" (Variables|Stats|GetStackSize) (Variables|Default|GetTagData))))

(fn DecompressfromStack
  (params (ItemStack :type Item%20Stack%20Structure))
  (bind (_stacksize _tagdata) (Utilities|Struct|BreakItemStack ItemStack))
  (Variables|Default|SetTagData _tagdata)
  (Variables|Stats|SetStackSize _stacksize)
  (CallFunction|DecompressTags _tagdata))

(fn DamageEntity
  (params (Location :type Vector :default "0, 0, 0") (Component :type Primitive%20Component%20Object%20Reference) (Damage :type Weapon%20Damage%20Structure) (Damager :type Actor%20Object%20Reference) (EquipmentSlot :type EquipmentSlot%20Enum :default "NewEnumerator0"))
  (return false))

(fn GetContextActions
  (params (Player :type RPG%20Character%20Object%20Reference))
  (return (Variables|Default|GetContextAction)))

(fn GetDisplayText
  (bind _itemdisplayname (Variables|Display|GetItemDisplayName))
  (bind _stacksize (Variables|Stats|GetStackSize))
  (if (> _stacksize 1)
    (return (Utilities|Text|ToText(String) (Utilities|String|Append (Utilities|String|ToString(Text) _itemdisplayname) " (" (Utilities|String|ToString(Integer) _stacksize) ")")))
    (else
      (return _itemdisplayname))))

(fn GetIneractable
  (return true))