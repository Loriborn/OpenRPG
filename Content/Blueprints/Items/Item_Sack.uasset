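; Item_Sack is an RPG item Blueprint for a sack container that can be inspected, picked up, equipped or opened.
; It initializes its InventoryComponent on the server at BeginPlay and exposes its available actions through GetContextActions.
; PerformAction dispatches the chosen action, with opening showing the sack's inventory through the user's RPGPlayerController and registering that character as interacting with it.
; Inspect only prints a placeholder string.
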(event EventPerformAction
  (params (User :type Actor%20Object%20Reference) (Action :type Name :default "None"))
  (bind _asrpgcharacter (Utilities|Casting|CastToRPGCharacter User))
  (bind _inventorycomponent (Variables|Default|GetInventoryComponent))
  (switch name Action
    (:inspect
      (Development|PrintString "looks like a thing"))
    (:pickup
      (CallFunction|PickupItem User))
    (:equip
      (CallFunction|EquipItem User))
    (:open_c
      (Default|OpenInventory (.AsRPGPlayer%20Controller (Utilities|Casting|CastToRPGPlayerController (Pawn|GetController _asrpgcharacter))) _inventorycomponent false)
      (Default|ToggleCharacterInteraction _inventorycomponent _asrpgcharacter true))))

(event EventBeginPlay
  (Networking|SwitchHasAuthority
    (:Authority
      (Default|InitializeInventory (Variables|Default|GetInventoryComponent)))))

(fn ConstructionScript
  (|CallParentFunction))

(fn GetContextActions
  (params (Player :type RPG%20Character%20Object%20Reference))
  (return (Variables|Default|GetContextAction)))