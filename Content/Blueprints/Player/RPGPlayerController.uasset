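; RPG player controller that handles cursor-driven interaction, the HUD and inventory windows.
; Holding ShowCursor enables mouse mode, with a looping timer feeding cursor direction to the character.
; Tick traces under the cursor to set the look-at object and hand cursor, and pins the mouse while rotating grabbed objects.
; Right-click opens context menus on interactables, while Send events forward item and container requests to inventories.
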(event Custom|PassMouseDirection
  (bind (_locationx _locationy) (Game|Player|GetMousePosition))
  (bind _returnvalue (Pawn|GetControlledPawn))
  (bind _asrpgcharacter (Utilities|Casting|CastToRPGCharacter _returnvalue))
  (if (not (Variables|/Game/Blueprints/Player/RPGCharacter.RPGCharacter_C|GetGrabbedObjectRotating _asrpgcharacter))
    (Default|UpdateMouseForwardVector _asrpgcharacter (.WorldDirection (Class|PlayerController|DeprojectScreenPositiontoWorld _locationx _locationy)))))

(event Custom|SetupMouseDirectionTimer
  (params (NewState :type Boolean))
  (if NewState
    (bind _returnvalue (Utilities|Time|SetTimerbyEvent (delegate Custom|PassMouseDirection) 0.05 true))
    (Variables|Default|SetMouseTimer _returnvalue)
    (Default|UpdateMouseForwardVector (.AsRPGCharacter (Utilities|Casting|CastToRPGCharacter (Pawn|GetControlledPawn))) (Math|Vector|GetForwardVector (Pawn|GetControlRotation :!class /Script/Engine.Controller)))
    (else
      (Utilities|Time|ClearandInvalidateTimerbyHandle (Variables|Default|GetMouseTimer)))))

(event Custom|ToggleCursor
  (params (NewState :type Boolean))
  (bind _returnvalue (Viewport|GetViewportSize))
  (bind _self self)
  (bind _hudreference (Variables|Default|GetHUDReference))
  ;[0.2249 0.4679 1] Toggle mouse view whenever key is pressed; when toggled on, show cursor, enable mouse in HUD, and ensure game & UI are active (center mouse too)
  (Class|PlayerController|SetMouseLocation (/ (Math|Float|Truncate (.x _returnvalue)) 2) (/ (Math|Float|Truncate (.y _returnvalue)) 2))
  (if NewState
    (Variables|Default|SetbShowMouseCursor true)
    (Input|SetInputModeGameandUI _self 0 "LockAlways" false)
    (bind _output_get (Variables|Default|SetMouseMode true))
    (Default|ToggleMouseMode _hudreference _output_get)
    (else
      (ContextMenu|CloseAllWindows)
      (Variables|Default|SetbShowMouseCursor false)
      (Input|SetInputModeGameOnly _self)
      (bind _output_get_2 (Variables|Default|SetMouseMode false))
      (Default|ToggleMouseMode _hudreference _output_get_2)
      (Utilities|Set|Clear (Variables|Default|GetMouseBlockers))))
  (Default|ToggleMouseModeServer (.AsRPGCharacter (Utilities|Casting|CastToRPGCharacter (Pawn|GetControlledPawn))) (Variables|Default|GetMouseMode))
  (CallFunction|SetupMouseDirectionTimer (Variables|Default|GetMouseMode)))

(event Custom|SendSplitStackRequest
  (params (Inventory :type Inventory%20Component%20Object%20Reference) (Index :type Integer) (IsSingle :type Boolean))
  (Default|SplitItemStack Inventory Index IsSingle))

(event Custom|LockMouseEvent
  (bind (_locationx _locationy) (Game|Player|GetMousePosition))
  (Variables|Default|SetLockMouseTo (Math|Vector2D|MakeVector2D _locationx _locationy)))

(event Custom|OpenInventory
  (params (Inventory :type Inventory%20Component%20Object%20Reference) (Internal :type Boolean))
  (bind _alreadyopen (ContextMenu|CheckforOpenInventory Inventory))
  (if (not _alreadyopen)
    (UI|CreateInventoryScreen Inventory Internal)))

(event Custom|SendDropItemRequest
  (params (Inventory :type Inventory%20Component%20Object%20Reference) (StackIndex :type Integer) (Vector :type Vector))
  (Default|DropItemStack Inventory StackIndex Vector))

(event Custom|SendTransferItemRequest
  (params (Stack :type Item%20Stack%20Structure) (Index :type Integer) (FromInventory :type Inventory%20Component%20Object%20Reference) (ToInventory :type Inventory%20Component%20Object%20Reference))
  (Default|RemoveItemStack FromInventory Index)
  (Default|AddItemStackfromItemStack ToInventory Stack false))

(event Custom|SendCloseContainerRequest
  (params (Inventory :type Inventory%20Component%20Object%20Reference))
  (Default|ToggleCharacterInteraction Inventory (.AsRPGCharacter (Utilities|Casting|CastToRPGCharacter (Pawn|GetControlledPawn))) false))

(event Custom|SendMoveItemRequest
  (params (Inventory :type Inventory%20Component%20Object%20Reference) (Index :type Integer) (NewLocation :type Vector%202D%20Structure) (MergeIndex :type Integer))
  (Default|MoveItemStack Inventory Index NewLocation MergeIndex))

(event EventBeginPlay
  (UI|CreateHUD))

(event EventTick
  (params (DeltaSeconds :type Float%20%28single-precision%29))
  ;[1 1 1] Tick!
  (Interaction|LookatTrace)
  (Interaction|LockMouse))

(event Input|ActionEvents|InputActionShowCursor
  (params (Key :type Key%20Structure))
  ;[0.2249 0.4679 1] Toggle mouse view whenever key is pressed; when toggled on, show cursor, enable mouse in HUD, and ensure game & UI are active (center mouse too)
  (:Pressed
    (CallFunction|ToggleCursor true))
  (:Released
    (CallFunction|ToggleCursor false)))

(event Input|MouseEvents|RightMouseButton
  (params (Key :type Key%20Structure))
  (:Pressed
    (ContextMenu|CreateContextMenu)))

(fn ConstructionScript)

(fn CreateClientTrace
  (params (ActorsToIgnore :type Array%20of%20Actor%20Object%20References) (Distance :type Float%20%28single-precision%29) (StartLocation :type Vector%202D%20Structure))
  (bind (_worldlocation _worlddirection) (Class|PlayerController|DeprojectScreenPositiontoWorld (.x StartLocation) (.y StartLocation)))
  (bind _returnvalue (* _worlddirection Distance))
  (bind _returnvalue_2 (+ _worldlocation _returnvalue))
  (bind (_outhit _returnvalue_3) (Collision|LineTraceByChannel _worldlocation _returnvalue_2 "TraceTypeQuery1" false ActorsToIgnore "None"))
  (return _outhit _returnvalue_3 _returnvalue_2))

(fn LookatTrace
  (bind _returnvalue (Pawn|GetControlledPawn))
  (bind (_locationx _locationy) (Game|Player|GetMousePosition))
  (bind _asrpgcharacter (Utilities|Casting|CastToRPGCharacter _returnvalue))
  (if (Pawn|IsLocalController)
    (if (Variables|Default|GetMouseMode)
      (if (> (Utilities|Set|Length (Variables|Default|GetMouseBlockers)) 0)
        (Utilities|IsValid (Variables|/Game/Blueprints/Player/RPGCharacter.RPGCharacter_C|GetRecentLookedObject _asrpgcharacter)
          (:Is%20Valid
            (Default|SetLookatObject :self _asrpgcharacter)))
        (else
          (bind (_hit _success) (Interaction|CreateClientTrace (Utilities|Array|MakeArray _returnvalue) 3e+02 (Math|Vector2D|MakeVector2D _locationx _locationy)))
          (bind _isinteractable (Default|SetLookatObject _asrpgcharacter _hit _success))
          (Utilities|IsValid (Variables|Default|GetGrabbedWidget)
            (:Is%20Not%20Valid
              (Interaction|InteractableSetCursor _isinteractable))))))))

(fn InteractableSetCursor
  (params (Interactable :type Boolean))
  (bind (_locationx _locationy) (Game|Player|GetMousePosition))
  (Utilities|IsValid (Variables|/Game/Blueprints/Player/RPGCharacter.RPGCharacter_C|GetGrabbedComponent (.AsRPGCharacter (Utilities|Casting|CastToRPGCharacter (Pawn|GetControlledPawn))))
    (:Is%20Valid
      (if (not (Utilities|Enum|Equal(Enum) (Variables|Default|GetCurrentMouseCursor) "GrabHandClosed"))
        (Variables|Default|SetCurrentMouseCursor "GrabHandClosed")
        ;[1 1 1] if we don't simulate mouse movement, it won't update cursor until mouse is moved
        (Class|PlayerController|SetMouseLocation (Math|Float|Truncate _locationx) (Math|Float|Truncate _locationy) :!label _label)))
    (:Is%20Not%20Valid
      (if Interactable
        (if (not (Utilities|Enum|Equal(Enum) (Variables|Default|GetCurrentMouseCursor) "GrabHand"))
          (Variables|Default|SetCurrentMouseCursor "GrabHand")
          (goto _label))
        (elif (not (Utilities|Enum|Equal(Enum) (Variables|Default|GetCurrentMouseCursor) "Default"))
          (Variables|Default|SetCurrentMouseCursor "Default")
          (goto _label))))))

(fn LockMouse
  (bind _returnvalue (Pawn|GetControlledPawn))
  (bind _lockmouseto (Variables|Default|GetLockMouseTo))
  (bind _asrpgcharacter (Utilities|Casting|CastToRPGCharacter _returnvalue))
  (if (Pawn|IsLocalController)
    (Utilities|IsValid _asrpgcharacter
      (:Is%20Valid
        (if (Variables|/Game/Blueprints/Player/RPGCharacter.RPGCharacter_C|GetGrabbedObjectRotating _asrpgcharacter)
          (Class|PlayerController|SetMouseLocation (Math|Float|Truncate (.x _lockmouseto)) (Math|Float|Truncate (.y _lockmouseto))))))))

(fn CreateHUD
  (if (Pawn|IsLocalController)
    (bind _returnvalue (UserInterface|CreateWidget "/Game/Blueprints/UI/UI_HUD.UI_HUD_C" self))
    (UserInterface|Viewport|AddtoViewport _returnvalue 0)
    (Variables|Default|SetHUDReference _returnvalue)
    (UI|CreateInventoryScreen (Variables|/Game/Blueprints/Player/RPGCharacter.RPGCharacter_C|GetInventory (.AsRPGCharacter (Utilities|Casting|CastToRPGCharacter (Pawn|GetControlledPawn)))) true)))

(fn CreateContextMenu
  (bind _returnvalue (Pawn|GetControlledPawn))
  (bind _asrpgcharacter (Utilities|Casting|CastToRPGCharacter _returnvalue))
  (bind _recentlookedobject (Variables|/Game/Blueprints/Player/RPGCharacter.RPGCharacter_C|GetRecentLookedObject _asrpgcharacter))
  (if (Pawn|IsLocalController)
    (bind _canopen (ContextMenu|CheckCMOpenable))
    (if _canopen
      (bind _foundwidgets (Widget|GetAllWidgetsOfClass "/Game/Blueprints/UI/UI_ContextMenu.UI_ContextMenu_C" false))
      (for _array_element _foundwidgets
        (if (Widget|IsVisible _array_element)
          (if (== (Variables|/Game/Blueprints/UI/UI_ContextMenu.UI_ContextMenu_C|GetContextActor _array_element) _recentlookedobject)
            (Default|CloseWindow (Variables|/Game/Blueprints/UI/UI_ContextMenu.UI_ContextMenu_C|GetOwnerPanel _array_element)))))
      (bind _vectoroffset (Interaction|SetInteractionWV))
      (bind _text (Class|IInteractableEntity|GetDisplayText(Message) _recentlookedobject))
      (bind _returnvalue_2 (UserInterface|CreateWidget "/Game/Blueprints/UI/UI_WindowsPanel.UI_WindowsPanel_C" self))
      (Widget|Panel|AddChild (Variables|/Game/Blueprints/UI/UI_HUD.UI_HUD_C|GetViewportPanel (Variables|Default|GetHUDReference)) _returnvalue_2)
      (Default|ConstructPanel _returnvalue_2 _text "/Game/Blueprints/UI/UI_ContextMenu.UI_ContextMenu_C" true "(X=256.000000,Y=256.000000)" false _recentlookedobject _vectoroffset true)
      (Default|ConstructPanel (.AsUI%20Context%20Menu (Utilities|Casting|CastToUI_ContextMenu (Variables|/Game/Blueprints/UI/UI_WindowsPanel.UI_WindowsPanel_C|GetSubWidget _returnvalue_2))) _recentlookedobject _returnvalue_2))))

(fn CheckCMOpenable
  (bind _returnvalue (Pawn|GetControlledPawn))
  (bind _asrpgcharacter (Utilities|Casting|CastToRPGCharacter _returnvalue))
  (bind _recentlookedobject (Variables|/Game/Blueprints/Player/RPGCharacter.RPGCharacter_C|GetRecentLookedObject _asrpgcharacter))
  (if (Variables|Default|GetMouseMode)
    (if (not (> (Utilities|Set|Length (Variables|Default|GetMouseBlockers)) 0))
      (Utilities|IsValid (Variables|/Game/Blueprints/Player/RPGCharacter.RPGCharacter_C|GetGrabbedComponent _asrpgcharacter)
        (:Is%20Not%20Valid
          (Utilities|IsValid _recentlookedobject
            (:Is%20Valid
              (bind _contextactions (Class|IInteractableEntity|GetContextActions(Message) _recentlookedobject _asrpgcharacter))
              (bind _keys (Utilities|Map|Keys _contextactions))
              (if (!= (Utilities|Array|Length _keys) 0)
                (bind _canopencm (Class|IInteractableEntity|GetIneractable(Message) _recentlookedobject))
                (return _canopencm)))))))))

(fn SetInteractionWV
  (bind (_locationx _locationy) (Game|Player|GetMousePosition))
  (bind (_hit _success _endlocation) (Interaction|CreateClientTrace (Utilities|Array|MakeArray (Pawn|GetControlledPawn)) 3e+02 (Math|Vector2D|MakeVector2D _locationx _locationy)))
  (if _success
    (return (- (.Location (Collision|BreakHitResult _hit)) (Transformation|GetActorLocation (.HitActor (Collision|BreakHitResult _hit)))))
    (else
      (return _endlocation))))

(fn CreateInventoryScreen
  (params (LinkedInventory :type Inventory%20Component%20Object%20Reference) (InternalInventory :type Boolean))
  (if (Pawn|IsLocalController)
    (bind _returnvalue (UserInterface|CreateWidget "/Game/Blueprints/UI/UI_WindowsPanel.UI_WindowsPanel_C" self))
    (Widget|Panel|AddChild (Variables|/Game/Blueprints/UI/UI_HUD.UI_HUD_C|GetViewportPanel (Variables|Default|GetHUDReference)) _returnvalue)
    (if InternalInventory
      _
      (else
        (LocalVariables|SetActor (Components|GetOwner LinkedInventory))))
    (Default|ConstructPanel _returnvalue "Inventory" "/Game/Blueprints/UI/UI_Inventory.UI_Inventory_C" false "(X=512.000000,Y=512.000000)" true (LocalVariables|GetActor) "0, 0, 0" false)
    (Variables|/Game/Blueprints/UI/UI_Inventory.UI_Inventory_C|SetLinkedInventory (.AsUI%20Inventory (Utilities|Casting|CastToUI_Inventory (Variables|/Game/Blueprints/UI/UI_WindowsPanel.UI_WindowsPanel_C|GetSubWidget _returnvalue))) LinkedInventory)
    (Default|PopulatePanel (.AsUI%20Inventory (Utilities|Casting|CastToUI_Inventory (Variables|/Game/Blueprints/UI/UI_WindowsPanel.UI_WindowsPanel_C|GetSubWidget _returnvalue))))
    (Variables|/Game/Blueprints/UI/UI_Inventory.UI_Inventory_C|SetOwnerPanel (.AsUI%20Inventory (Utilities|Casting|CastToUI_Inventory (Variables|/Game/Blueprints/UI/UI_WindowsPanel.UI_WindowsPanel_C|GetSubWidget _returnvalue))) _returnvalue)
    (Variables|/Game/Blueprints/UI/UI_Inventory.UI_Inventory_C|SetBackgroundImage (.AsUI%20Inventory (Utilities|Casting|CastToUI_Inventory (Variables|/Game/Blueprints/UI/UI_WindowsPanel.UI_WindowsPanel_C|GetSubWidget _returnvalue))) (Variables|/Game/Blueprints/Components/InventoryComponent.InventoryComponent_C|GetBackgroundImage LinkedInventory))))

(fn CloseAllWindows
  (bind _foundwidgets (Widget|GetAllWidgetsOfClass "/Game/Blueprints/UI/UI_WindowsPanel.UI_WindowsPanel_C" false))
  (for _array_element _foundwidgets
    (if (Widget|IsVisible _array_element)
      (if (Variables|/Game/Blueprints/UI/UI_WindowsPanel.UI_WindowsPanel_C|GetCloseOnMouseExit _array_element)
        (Default|CloseWindow _array_element)))))

(fn CheckforOpenInventory
  (params (LinkedInventory :type Inventory%20Component%20Object%20Reference))
  (bind _foundwidgets (Widget|GetAllWidgetsOfClass "/Game/Blueprints/UI/UI_Inventory.UI_Inventory_C" false))
  (bind _array_element (Utilities|Array|ForEachLoopwithBreak _foundwidgets :!label _label)
    (:LoopBody
      (if (and (== LinkedInventory (Variables|/Game/Blueprints/UI/UI_Inventory.UI_Inventory_C|GetLinkedInventory _array_element)) (Widget|IsVisible _array_element))
        (LocalVariables|SetFound true)
        (goto _label Break)))
    (:Completed
      (return (LocalVariables|GetFound)))))

(fn SetPPSettings)